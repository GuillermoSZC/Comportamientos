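; AI controller that sends its AI_Character pawn wandering between the Waypoint actors it is allowed to use.
; On BeginPlay it gathers waypoints whose AllowedAccess contains the pawn, appends them to Routes, shuffles and moves to the first.
; Each completed move, whatever the result, repeats this after a short delay, and Routes is never cleared between passes.
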(event Custom|MoveCompleted_Event_0
  (params (RequestID :type AI%20Request%20ID%20Structure) (Result :type EPathFollowingResult%20Enum :default "Success"))
  (bind _routes (Variables|Default|GetRoutes))
  ;[0.4248 1 0.4767] Parte 1
  (Utilities|FlowControl|Delay 3.0)
  (bind _outactors (Actor|GetAllActorsOfClass "/Game/Blueprints/Waypoint.Waypoint_C"))
  (bind _asai_character (Utilities|Casting|CastToAI_Character (Pawn|GetControlledPawn)))
  (for _array_element _outactors
    (if (!= (Utilities|Array|FindItem (Variables|/Game/Blueprints/Waypoint.Waypoint_C|GetAllowedAccess _array_element) _asai_character) -1)
      (Utilities|Array|Add (Variables|Default|GetRoutes) _array_element)))
  (Utilities|Array|Shuffle _routes)
  (AI|Navigation|MovetoActor (Utilities|Array|Get(acopy) _routes) -1.0 true true true 0))

(event EventBeginPlay
  (bind _routes (Variables|Default|GetRoutes))
  ;[0.4248 1 0.4767] Parte 1
  (EventDispatchers|BindEventtoReceiveMoveCompleted (delegate Custom|MoveCompleted_Event_0))
  (bind _outactors (Actor|GetAllActorsOfClass "/Game/Blueprints/Waypoint.Waypoint_C"))
  (bind _asai_character (Utilities|Casting|CastToAI_Character (Pawn|GetControlledPawn)))
  (for _array_element _outactors
    (if (!= (Utilities|Array|FindItem (Variables|/Game/Blueprints/Waypoint.Waypoint_C|GetAllowedAccess _array_element) _asai_character) -1)
      (Utilities|Array|Add (Variables|Default|GetRoutes) _array_element)))
  (Utilities|Array|Shuffle _routes)
  (AI|Navigation|MovetoActor (Utilities|Array|Get(acopy) _routes) -1.0 true true true 0))

(fn ConstructionScript)